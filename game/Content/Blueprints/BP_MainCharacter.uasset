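; Player character for a timed delivery game: carry food to random room numbers for points, or help Samo deliver chairs to raise the score multiplier.
; Overlapped "Interact" actors answer message calls that drive pickups, deliveries and dialogue, which pauses the countdown (handle misleadingly named TripOverTimer).
; A looping timer flags trips while carrying; moving then starts a timeline-driven slider skill check, and failure drops the load.
; Countdown expiry freezes time and shows game over.
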(event OnComponentBeginOverlap(CapsuleComponent)
  (params (OverlappedComponent :type Primitive%20Component%20Object%20Reference) (OtherActor :type Actor%20Object%20Reference) (OtherComp :type Primitive%20Component%20Object%20Reference) (OtherBodyIndex :type Integer) (bFromSweep :type Boolean) (SweepResult :type Hit%20Result%20Structure%20%28by%20ref%29))
  (if (Actor|ActorHasTag OtherActor "Interact")
    (Variables|Default|SetInteractPlace OtherActor)
    (Variables|Default|SetcanInteract true)))

(event OnComponentEndOverlap(CapsuleComponent)
  (params (OverlappedComponent :type Primitive%20Component%20Object%20Reference) (OtherActor :type Actor%20Object%20Reference) (OtherComp :type Primitive%20Component%20Object%20Reference) (OtherBodyIndex :type Integer))
  (if (Actor|ActorHasTag OtherActor "Interact")
    (Variables|Default|SetcanInteract false)))

(event Custom|Timer
  (bind _returnvalue (Game|GetPlayerController 0))
  (bind _hudko (Variables|Default|Gethudko))
  (if (== (Variables|Default|Gettime) 0)
    (Rendering|Components|TextRender|SetText (Variables|/Game/UI/HUD.HUD_C|GetScoreText _hudko) (Utilities|Text|ToText(String) (Utilities|String|Append "Your score was : " (Utilities|String|ToString(Float) (Variables|Default|Getpoints)))))
    (Widget|SetVisibility (Variables|/Game/UI/HUD.HUD_C|GetBlackScreen _hudko) "Visible")
    (Variables|/Script/Engine.PlayerController|SetbShowMouseCursor _returnvalue true)
    (Input|SetInputModeUIOnly _returnvalue 0 "DoNotLock" false)
    (Utilities|Time|SetGlobalTimeDilation 0.0)
    (else
      (Rendering|Components|TextRender|SetText (Variables|/Game/UI/HUD.HUD_C|GetTimerText (Variables|Default|Gethudko)) (Utilities|Text|ToText(String) (Utilities|String|Append "Koniec prestávky : " (Utilities|String|ToString(Integer) (- (Variables|Default|Gettime) 1)))))
      (Math|Integer|DecrementInt (Variables|Default|Gettime)))))

(event Custom|TripOver
  (if (not (Variables|Default|GetisDoingSkillCheck))
    (if (or (Variables|Default|GethaveFood) (Variables|Default|GethaveChair))
      (if (not (Variables|Default|GetcanInteract))
        (Variables|Default|SettripedOver true)))))

(event Input|EnhancedActionEvents|EnhancedInputActionIA_Interact
  (params (ActionValue :type Boolean) (ElapsedSeconds :type Float%20%28double-precision%29) (TriggeredSeconds :type Float%20%28double-precision%29) (InputAction :type Input%20Action%20Object%20Reference :default "/Game/Blueprints/Input/IA_Interact.IA_Interact"))
  (bind _returnvalue (Game|GetPlayerController 0))
  (bind _hudko (Variables|Default|Gethudko))
  (bind _skillcheckgreenarea (Variables|/Game/UI/HUD.HUD_C|GetSkillCheckGreenArea _hudko))
  (bind _skillcheckslilder (Variables|/Game/UI/HUD.HUD_C|GetSkillCheckSlilder _hudko))
  (bind _returnvalue_2 (Class|WidgetLayoutLibrary|SlotasCanvasSlot _skillcheckgreenarea))
  (bind _returnvalue_3 (Class|WidgetLayoutLibrary|SlotasCanvasSlot _skillcheckslilder))
  (bind _returnvalue_4 (Class|CanvasPanelSlot|GetPosition _returnvalue_2))
  (bind _returnvalue_5 (Class|CanvasPanelSlot|GetPosition _returnvalue_3))
  (bind _returnvalue_6 (Class|CanvasPanelSlot|GetSize _returnvalue_2))
  (bind _returnvalue_7 (Class|CanvasPanelSlot|GetSize _returnvalue_3))
  (bind _returnvalue_8 (/ (.x _returnvalue_6) 2.0))
  (bind _returnvalue_9 (/ (.x _returnvalue_7) 2.0))
  (:Started
    (if (Variables|Default|GetisDoingSkillCheck)
      (if (or (>= (- (.x _returnvalue_5) _returnvalue_9) (+ (.x _returnvalue_4) _returnvalue_8)) (<= (+ (.x _returnvalue_5) _returnvalue_9) (- (.x _returnvalue_4) _returnvalue_8)))
        (Development|PrintString "netrafil")
        (CallFunction|TripOverFunc)
        (else
          (Development|PrintString "trafil")
          (Audio|Components|Audio|Stop (Variables|Default|GetSliderTimeline))
          (Audio|Components|Audio|Stop (Variables|Default|GetTimeline))))
      (Widget|SetVisibility (Variables|/Game/UI/HUD.HUD_C|GetSkillCheckText (Variables|Default|Gethudko)) "Collapsed")
      (Variables|Default|SetcanMove true)
      (Variables|Default|SetisDoingSkillCheck false)
      (Variables|Default|SettripedOver false)
      (elif (Variables|Default|GetcanInteract)
        (Development|PrintString "moze")
        (bind _isitsamo (Class|MyInterface|AreYouSamo(Message) (Variables|Default|GetInteractPlace)))
        (if _isitsamo
          (Variables|Default|SetcanMove false)
          (Widget|SetVisibility (Variables|/Game/UI/HUD.HUD_C|GetDialogueBox (Variables|Default|Gethudko)) "Visible")
          (Utilities|Time|PauseTimerbyHandle (Variables|Default|GetTripOverTimer))
          (Variables|/Script/Engine.PlayerController|SetbShowMouseCursor _returnvalue true)
          (Input|SetInputModeUIOnly _returnvalue 0 "DoNotLock" false)
          (Audio|PlaySoundatLocation "/Game/Sounds/SamoVoceLines.SamoVoceLines" "0, 0, 0" "0, 0, 0" 1.0 1.0 0.0 0 0 0 0)
          (else
            (bind _ispickup (Class|MyInterface|IsPickUp?(Message) (Variables|Default|GetInteractPlace)))
            (if _ispickup
              (if (not (Variables|Default|GethaveFood))
                (Variables|Default|SethaveFood true)
                (Rendering|SetVisibility (Variables|Default|Getfood) true false)
                (Variables|Default|SetroomNumber (.OutItem (Utilities|Array|Random (Variables|Default|GetroomNumberArray))))
                (Rendering|Components|TextRender|SetText (Variables|/Game/UI/HUD.HUD_C|GetRoomNumberText (Variables|Default|Gethudko)) (Utilities|Text|ToText(String) (Utilities|String|Append "Room number : " (Utilities|String|ToString(Integer) (Variables|Default|GetroomNumber))))))
              (elif (Variables|Default|GethaveFood)
                (bind _num (Class|MyInterface|GetRoomNumber(Message) (Variables|Default|GetInteractPlace)))
                (if (== _num (Variables|Default|GetroomNumber))
                  (Variables|Default|SethaveFood false)
                  (Rendering|SetVisibility (Variables|Default|Getfood) false false)
                  (Variables|Default|Setpoints (+ (Variables|Default|Getpoints) (* (Variables|Default|GetpointsMultiplayer) 1e+02)))
                  (Rendering|Components|TextRender|SetText (Variables|/Game/UI/HUD.HUD_C|GetPointsText (Variables|Default|Gethudko)) (Utilities|Text|ToText(String) (Utilities|String|Append "Points: " (Utilities|String|ToString(Float) (Variables|Default|Getpoints)))))
                  (Rendering|Components|TextRender|SetText (Variables|/Game/UI/HUD.HUD_C|GetRoomNumberText (Variables|Default|Gethudko)) "Room number : "))
                (elif (Variables|Default|GethaveChair)
                  (bind _num_2 (Class|MyInterface|GetRoomNumber(Message) (Variables|Default|GetInteractPlace)))
                  (if (== _num_2 (Variables|Default|GetroomNumber))
                    (Variables|Default|SethaveChair false)
                    (Rendering|SetVisibility (Variables|Default|GetChair) false false)
                    (Variables|Default|SetpointsMultiplayer (+ (Variables|Default|GetpointsMultiplayer) 0.2))
                    (Rendering|Components|TextRender|SetText (Variables|/Game/UI/HUD.HUD_C|GetMultiplayer (Variables|Default|Gethudko)) (Utilities|Text|ToText(String) (Utilities|String|Append "Multiplayer : " (Utilities|String|ToString(Float) (Variables|Default|GetpointsMultiplayer)))))
                    (Rendering|Components|TextRender|SetText (Variables|/Game/UI/HUD.HUD_C|GetRoomNumberText (Variables|Default|Gethudko)) "Room number : ")))))))
        (else
          (Development|PrintString "nemoze"))))))

(event Input|EnhancedActionEvents|EnhancedInputActionIA_Move
  (params (ActionValue :type Vector%202D%20Structure) (ElapsedSeconds :type Float%20%28double-precision%29) (TriggeredSeconds :type Float%20%28double-precision%29) (InputAction :type Input%20Action%20Object%20Reference :default "/Game/Blueprints/Input/IA_Move.IA_Move"))
  (bind _hudko (Variables|Default|Gethudko))
  (bind _skillcheckbase (Variables|/Game/UI/HUD.HUD_C|GetSkillCheckBase _hudko))
  (bind _skillcheckslilder (Variables|/Game/UI/HUD.HUD_C|GetSkillCheckSlilder _hudko))
  (bind _returnvalue (Class|WidgetLayoutLibrary|SlotasCanvasSlot _skillcheckbase))
  (bind _returnvalue_2 (Class|WidgetLayoutLibrary|SlotasCanvasSlot _skillcheckslilder))
  (bind _returnvalue_3 (Class|CanvasPanelSlot|GetSize _returnvalue))
  (bind _returnvalue_4 (/ (.x _returnvalue_3) 2.0))
  (bind _returnvalue_5 (- _returnvalue_4 24.0))
  (if (Variables|Default|GetcanMove)
    (if (Variables|Default|GettripedOver)
      (Variables|Default|SetcanMove false)
      (Variables|Default|SetisDoingSkillCheck true)
      (Class|CanvasPanelSlot|SetPosition _returnvalue_2 (Math|Vector2D|MakeVector2D -2.6e+02 0.0))
      (Class|CanvasPanelSlot|SetPosition (Class|WidgetLayoutLibrary|SlotasCanvasSlot (Variables|/Game/UI/HUD.HUD_C|GetSkillCheckGreenArea _hudko)) (Math|Vector2D|MakeVector2D (Math|Random|RandomFloatinRange (* _returnvalue_5 -1.0) _returnvalue_5) 0.0))
      (Widget|SetVisibility _skillcheckbase "Visible")
      (Audio|PlaySoundatLocation "/Game/Sounds/potknutie.potknutie" "0, 0, 0" "0, 0, 0" 1.0 1.0 0.0 0 0 0 0)
      (bind _sliderposition (Timeline|SliderTimeline PlayFromStart)
        (:Update
          (Class|CanvasPanelSlot|SetPosition _returnvalue_2 (Math|Vector2D|MakeVector2D (Math|Float|Lerp -2.6e+02 2.6e+02 _sliderposition) 0.0)))
        (:Finished
          (bind _sliderposition_2 (Timeline|Timeline ReverseFromEnd)
            (:Update
              (Class|CanvasPanelSlot|SetPosition _returnvalue_2 (Math|Vector2D|MakeVector2D (Math|Float|Lerp -2.6e+02 2.6e+02 _sliderposition_2) 0.0)))
            (:Finished
              (CallFunction|TripOverFunc)))))
      (else
        (Pawn|Input|AddMovementInput (Transformation|GetActorRightVector) (.x ActionValue) false)
        (Pawn|Input|AddMovementInput (Transformation|GetActorForwardVector) (.y ActionValue) false)))))

(event Input|EnhancedActionEvents|EnhancedInputActionIA_Look
  (params (ActionValue :type Vector%202D%20Structure) (ElapsedSeconds :type Float%20%28double-precision%29) (TriggeredSeconds :type Float%20%28double-precision%29) (InputAction :type Input%20Action%20Object%20Reference :default "/Game/Blueprints/Input/IA_Look.IA_Look"))
  (Pawn|Input|AddControllerYawInput (.x ActionValue))
  (Pawn|Input|AddControllerPitchInput (.y ActionValue)))

(event EventBeginPlay
  (bind _returnvalue (Game|GetPlayerController 0))
  (CallFunction|SetupMappingContext)
  (bind _returnvalue_2 (UserInterface|CreateWidget "/Game/UI/HUD.HUD_C"))
  (bind _output_get (Variables|Default|Sethudko _returnvalue_2))
  (UserInterface|Viewport|AddtoViewport _output_get 0)
  (Variables|/Script/Engine.PlayerController|SetbShowMouseCursor _returnvalue false)
  (Input|SetInputModeGameOnly _returnvalue false)
  (bind _returnvalue_3 (Utilities|Time|SetTimerbyEvent (delegate Custom|Timer) 1.0 true))
  (Variables|Default|SetTripOverTimer _returnvalue_3)
  (Utilities|Time|SetTimerbyEvent (delegate Custom|TripOver) (Math|Random|RandomFloatinRange 5.0 15.0) true))

(event EventIWillHelp
  (bind _returnvalue (Game|GetPlayerController 0))
  (Variables|Default|SetcanMove true)
  (Variables|Default|SetcanInteract false)
  (Widget|SetVisibility (Variables|/Game/UI/HUD.HUD_C|GetDialogueBox (Variables|Default|Gethudko)) "Collapsed")
  (Rendering|SetVisibility (Variables|Default|GetChair) true false)
  (Variables|/Script/Engine.PlayerController|SetbShowMouseCursor _returnvalue false)
  (Input|SetInputModeGameOnly _returnvalue false)
  (Variables|Default|SethaveChair true)
  (Variables|Default|SetroomNumber (.OutItem (Utilities|Array|Random (Variables|Default|GetroomNumberArray))))
  (Rendering|Components|TextRender|SetText (Variables|/Game/UI/HUD.HUD_C|GetRoomNumberText (Variables|Default|Gethudko)) (Utilities|Text|ToText(String) (Utilities|String|Append "Room number : " (Utilities|String|ToString(Integer) (Variables|Default|GetroomNumber)))))
  (Utilities|Time|UnpauseTimerbyHandle (Variables|Default|GetTripOverTimer)))

(fn ConstructionScript
  (bind _charactermovement (Variables|Character|GetCharacterMovement))
  (Variables|/Script/Engine.CharacterMovementComponent|SetMaxWalkSpeed _charactermovement (* (Variables|/Script/Engine.CharacterMovementComponent|GetMaxWalkSpeed _charactermovement) (Variables|Default|GetCharacterSpeed))))

(fn SetupMappingContext
  (Input|AddMappingContext (PlayerController|LocalPlayerSubsystems|GetEnhancedInputLocalPlayerSubsystem (Game|GetPlayerController 0)) "/Game/Blueprints/Input/IMC_Default.IMC_Default" 0 "(bIgnoreAllPressedKeysUntilRelease=True,bForceImmediately=False,bNotifyUserSettings=False)"))

(fn TripOverFunc
  (Audio|Components|Audio|Stop (Variables|Default|GetSliderTimeline))
  (Audio|Components|Audio|Stop (Variables|Default|GetTimeline))
  (Rendering|SetVisibility (Variables|Default|Getfood) false false)
  (Rendering|SetVisibility (Variables|Default|GetChair) false false)
  (Variables|Default|SetcanMove true)
  (Variables|Default|SetisDoingSkillCheck false)
  (Variables|Default|SettripedOver false)
  (Variables|Default|SethaveFood false)
  (Variables|Default|SethaveChair false)
  (Rendering|Components|TextRender|SetText (Variables|/Game/UI/HUD.HUD_C|GetRoomNumberText (Variables|Default|Gethudko)) "Room number : ")
  (Game|SpawnActorfromClass "/Game/Blueprints/BP_DropedFood.BP_DropedFood_C" (Math|Transform|MakeTransform (Transformation|GetWorldLocation (Variables|Default|GetSpawnPoint)) "0, 0, 0" "1.000000,1.000000,1.000000") "Undefined" "MultiplyWithRoot" 0 0)
  (Audio|PlaySoundatLocation "/Game/Sounds/FoodDrop.FoodDrop" "0, 0, 0" "0, 0, 0" 1.0 1.0 0.0 0 0 0 0)
  (Widget|SetVisibility (Variables|/Game/UI/HUD.HUD_C|GetSkillCheckBase (Variables|Default|Gethudko)) "Collapsed"))

(fn AreYouSamo)

(fn GetRoomNumber
  (return 0))

(fn IsPickUp?
  (return false))