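; BP_BaseNPC is an NPC Blueprint, named as a base class, that shows a floating arrow indicator while the character is highlighted.
; Every Tick runs CheckHighlighted, which shows or hides the Arrow component according to IsHighlighted.
; While visible, the arrow bobs vertically by adding a sine of game time, scaled by FloatSpeed, to its current world Z each frame, so the travel depends on frame rate.
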(event EventTick
  (params (DeltaSeconds :type Float%20%28single-precision%29))
  (CallFunction|CheckHighlighted))

(fn ConstructionScript)

(fn CheckHighlighted
  (bind _arrow (Variables|Default|GetArrow))
  (bind _returnvalue (Transformation|GetWorldLocation _arrow))
  (if (Variables|Default|GetbIsHighlighted)
    (Development|SetHiddeninGame _arrow false false)
    (Transformation|SetWorldLocation _arrow (Math|Vector|MakeVector (.x _returnvalue) (.y _returnvalue) (+ (.z _returnvalue) (Math|Trig|Sin(Radians) (* (Utilities|Time|GetTimeSeconds) (Variables|Default|GetFloatSpeed))))) false false)
    (else
      (Development|SetHiddeninGame _arrow true false))))